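; BP_Prop is a breakable prop drawn with a Paper2D flipbook sprite that shatters when it takes any damage.
; The construction script shows the idle flipbook, and BeginPlay sets a state enum that gates damage so Break responds only while intact.
; Break plays the destroy flipbook, flips the state, then switches to the destroyed flipbook after a short fixed delay.
; A DropItem event is declared but empty.
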(event Custom|Break
  (bind _sprite (Variables|Default|GetSprite))
  ;[0.5234 1 0] Break Prop Action
  (Sprite|SetFlipbook _sprite (Variables|Default|GetAnimDestroy))
  (Components|Timeline|PlayfromStart _sprite)
  (Variables|Default|SetState "NewEnumerator0")
  (Utilities|FlowControl|Delay 0.4)
  (Sprite|SetFlipbook (Variables|Default|GetSprite) (Variables|Default|GetAnimDestroyed%20)))

(event Custom|DropItem)

(event EventBeginPlay
  (Variables|Default|SetState "NewEnumerator1"))

(event Game|Damage|EventAnyDamage
  (params (Damage :type Float%20%28single-precision%29) (DamageType :type Damage%20Type%20Object%20Reference) (InstigatedBy :type Controller%20Object%20Reference) (DamageCauser :type Actor%20Object%20Reference))
  ;[1 0.2344 0] Interface Communication
  (if (== (Variables|Default|GetState) 1)
    (CallFunction|Break)))

(fn ConstructionScript
  (Sprite|SetFlipbook (Variables|Default|GetSprite) (Variables|Default|GetAnimIdle)))