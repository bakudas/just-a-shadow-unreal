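; Core HUD Blueprint that creates the player's on-screen widgets and toggles menus such as the skill tree by name.
; BeginPlay sets game-only input, adds the main HUB widget to the viewport, then adds every widget registered in the WidgetList map.
; ToogleWidgetHUD forwards a key to ToogleSkillTree, which flips that map entry between Visible and Collapsed.
; The ToogleHUDWidgets function is an empty, unused stub.
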(event Custom|ToogleSkillTree
  (params (Key :type String%20%28by%20ref%29))
  (bind _widgetlist (Variables|Default|GetWidgetList))
  (bind _value (Utilities|Map|Find _widgetlist Key))
  (Utilities|IsValid _value
    (:Is%20Valid
      (switch Utilities|FlowControl|Switch|SwitchonESlateVisibility (Widget|GetVisibility _value)
        (:Visible
          (Widget|SetVisibility _value "Collapsed"))
        (:Collapsed
          (Widget|SetVisibility _value "Visible"))))))

(event EventBeginPlay
  (Utilities|FlowControl|Sequence
    (:then_0
      (Input|SetInputModeGameOnly (Game|Player|GetOwningPlayerController) true))
    (:then_1
      ;[0 0.8359 1] Handling with UI
      (bind _returnvalue (UserInterface|CreateWidget "/Game/UI/BP_HUB_Widget.BP_HUB_Widget_C" (Game|Player|GetOwningPlayerController)))
      (bind _output_get (Variables|Default|SetHUDWidget _returnvalue))
      (UserInterface|Viewport|AddtoViewport _output_get 0))
    (:then_2
      (bind _returnvalue_2 (UserInterface|CreateWidget "/Game/UI/WBP_Core_SkillTree_Menu.WBP_Core_SkillTree_Menu_C" (Game|Player|GetOwningPlayerController)))
      (Utilities|Map|Add (Variables|Default|GetWidgetList) "SkillTree" _returnvalue_2))
    (:then_3
      (bind _values (Utilities|Map|Values (Variables|Default|GetWidgetList)))
      (for _array_element _values
        (UserInterface|Viewport|AddtoViewport _array_element 0)))))

(event EventToogleWidgetHUD
  (params (WidgetName :type String))
  (CallFunction|ToogleSkillTree WidgetName))

(fn ConstructionScript)

(fn ToogleHUDWidgets
  (params (WidgetName :type String) (WidgetList :type Map%20of%20Strings%20to%20Objects)))