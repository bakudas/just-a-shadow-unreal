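; BP_Bullet is a projectile that damages any overlapped actor other than BP_Enemy, which suggests it is enemy fire.
; BulletMovimentAction sets local velocity from a direction and BulletSpeed, with gravity for Arc shots and none for Straight; Zig Zag currently behaves like Straight.
; A sphere overlap applies damage, and either that hit or a short lifetime timeout destroys the bullet and spawns BP_FireParticles.
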(event OnComponentBeginOverlap(SphereCollider)
  (params (OverlappedComponent :type Primitive%20Component%20Object%20Reference) (OtherActor :type Actor%20Object%20Reference) (OtherComp :type Primitive%20Component%20Object%20Reference) (OtherBodyIndex :type Integer) (bFromSweep :type Boolean) (SweepResult :type Hit%20Result%20Structure%20%28by%20ref%29))
  ;[0.8516 1 0] Hit Action
  (if (not (.bSuccess (Utilities|Casting|CastToBP_Enemy OtherActor)))
    (Game|Damage|ApplyDamage OtherActor 1.0 0 0 "/Script/Engine.DamageType")
    (Actor|DestroyActor)
    (Game|SpawnActorfromClass "/Game/Blueprints/BP_FireParticles.BP_FireParticles_C" (Math|Conversions|ToTransform(Vector) (.ImpactPoint (Collision|BreakHitResult SweepResult))) "Undefined" "OverrideRootScale" 0 0)))

(event Custom|BulletMovimentAction
  (params (NewVelocity :type Vector) (BulletMovimentType :type E_BulletMovimentType%20Enum :default "NewEnumerator1"))
  (bind _bulletmoviment (Variables|Default|GetBulletMoviment))
  ;[0.3594 1 0] Bullet Movement
  (Variables|Default|SetBulletDirection NewVelocity)
  (switch Utilities|FlowControl|Switch|SwitchonE_BulletMovimentType BulletMovimentType
    (:NewEnumerator1
      (Variables|/Script/Engine.ProjectileMovementComponent|SetProjectileGravityScale _bulletmoviment 0.5))
    (:NewEnumerator5
      (Variables|/Script/Engine.ProjectileMovementComponent|SetProjectileGravityScale _bulletmoviment 0.0 :!label _label))
    (:NewEnumerator6
      (goto _label)))
  (Game|Components|ProjectileMovement|SetVelocityinLocalSpace (Variables|Default|GetBulletMoviment) (* (Variables|Default|GetBulletSpeed) (Variables|Default|GetBulletDirection))))

(event EventBeginPlay
  ;[0 1 0.2031] Destroy overtime action
  (Utilities|FlowControl|Delay 3.0)
  (Game|SpawnActorfromClass "/Game/Blueprints/BP_FireParticles.BP_FireParticles_C" (Transformation|GetActorTransform) "Undefined" "OverrideRootScale" 0 0)
  (Actor|DestroyActor))

(event Collision|EventActorBeginOverlap
  (params (OtherActor :type Actor%20Object%20Reference)))

(event EventTick
  (params (DeltaSeconds :type Float%20%28single-precision%29)))

(fn ConstructionScript)