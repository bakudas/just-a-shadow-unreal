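; Paper2D tilemap actor that displays a level map and spawns an actor on matching tiles when play begins.
; The construction script assigns the Level tile map to the render component.
; BeginPlay scans every cell on layer 1 for tilesets whose name contains "TS_Tileset".
; Each match gets an actor spawned at its world-space tile center, nudged slightly along negative Y.
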(event EventBeginPlay
  (bind (_mapwidth _mapheight) (Class|PaperTileMapComponent|GetMapSize (Variables|Default|GetRenderComponent)))
  (for _index (range 0 (- _mapwidth 1))
    (for _index_2 (range 0 (- _mapheight 1))
      (if (Utilities|String|Contains (Utilities|GetDisplayName (.tileset (Class|PaperTileMapComponent|GetTile (Variables|Default|GetRenderComponent) _index _index_2 1))) "TS_Tileset" true)
        (Game|SpawnActorfromClass "/Game/Enemies/BP_Enemy_Child_Frag.BP_Enemy_Child_Frag_C" (Math|Transform|MakeTransform (+ (Class|PaperTileMapComponent|GetTileCenterPosition (Variables|Default|GetRenderComponent) _index _index_2 1 true) "0.000000,-2.000000,0.000000") "0, 0, 0" "1.000000,1.000000,1.000000") "Undefined" "MultiplyWithRoot" 0 0)))))

(fn ConstructionScript
  (Class|PaperTileMapComponent|SetTileMap (Variables|Default|GetRenderComponent) (Variables|Default|GetLevel)))