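; Gargoyle enemy Blueprint that breathes a burst of fire when the player enters its sight.
; A player overlapping the Sight component switches the Sprite to a one-shot fire flipbook.
; When that finishes, it spawns a fan of BP_FireParticles at SpawnPoint with increasing forward and upward local velocities, then returns to the looping idle flipbook.
; Sphere-trace debug nodes remain but never run.
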(event OnComponentBeginOverlap(Sight)
  (params (OverlappedComponent :type Primitive%20Component%20Object%20Reference) (OtherActor :type Actor%20Object%20Reference) (OtherComp :type Primitive%20Component%20Object%20Reference) (OtherBodyIndex :type Integer) (bFromSweep :type Boolean) (SweepResult :type Hit%20Result%20Structure%20%28by%20ref%29))
  (bind _sprite (Variables|Default|GetSprite))
  (Utilities|Casting|CastToBP_Core_Player OtherActor)
  (Sprite|SetFlipbook _sprite "/Game/Enemies/Animations/Gargoyle/FB_Gargoyle_Fire.FB_Gargoyle_Fire")
  (Components|Timeline|PlayfromStart _sprite)
  (Components|Timeline|SetLooping _sprite false))

(event OnFinishedPlaying(Sprite)
  (bind _sprite (Variables|Default|GetSprite))
  (for _index (range 0 10)
    (bind _returnvalue (Game|SpawnActorfromClass "/Game/Blueprints/BP_FireParticles.BP_FireParticles_C" (Math|Conversions|ToTransform(Vector) (Transformation|GetWorldLocation (Variables|Default|GetSpawnPoint))) "AlwaysSpawn" "OverrideRootScale" 0 0))
    (Game|Components|ProjectileMovement|SetVelocityinLocalSpace (Variables|/Game/Blueprints/BP_FireParticles.BP_FireParticles_C|GetProjectileMovement _returnvalue) (Math|Vector|MakeVector (Math|Conversions|ToFloat(Integer) (* (+ _index 1) 10)) 0.0 (Math|Conversions|ToFloat(Integer) (* (+ _index 1) 5)))))
  (Sprite|SetFlipbook _sprite "/Game/Enemies/Animations/Gargoyle/FB_Gargoyle_Idle.FB_Gargoyle_Idle")
  (Components|Timeline|PlayfromStart _sprite)
  (Components|Timeline|SetLooping _sprite true))

(event EventBeginPlay
  (|CallParentFunction))

(event Collision|EventActorBeginOverlap
  (params (OtherActor :type Actor%20Object%20Reference))
  (|CallParentFunction 0))

(event EventTick
  (params (DeltaSeconds :type Float%20%28single-precision%29))
  (|CallParentFunction DeltaSeconds))

(fn ConstructionScript
  (|CallParentFunction))