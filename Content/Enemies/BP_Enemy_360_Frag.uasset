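; BP_Enemy_360_Frag is a flipbook-sprite enemy that patrols along X and periodically fires through a child-actor BP_BulletSpawner.
; Tick feeds movement input, and a FlipFlop flips direction with a brief pause when it strays too far from its spawn point.
; If active, it attacks at BeginPlay and on a looping, randomly offset timer, halting movement while the attack flipbook plays and the spawner shoots.
; The Timeline-based movement is marked deprecated.
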(event OnFinishedPlaying(Sprite)
  ;[1 0 0.006586] Animation by Timeline (DEPRECATED)
)

(event Custom|Movement
  (bind _charactermovement (Variables|Character|GetCharacterMovement))
  (bind _charactermovement_2 (Variables|Character|GetCharacterMovement))
  (if (Variables|Default|GetbCanMove)
    (if (Variables|Default|GetbIsReversed)
      (Components|Movement|StopMovementImmediately _charactermovement_2)
      (Class|PawnMovementComponent|AddInputVector _charactermovement (Math|Vector|MakeVector -2.0 0.0 0.0) false)
      (else
        (Components|Movement|StopMovementImmediately _charactermovement_2)
        (Class|PawnMovementComponent|AddInputVector _charactermovement (Math|Vector|MakeVector 2.0 0.0 0.0) false)))
    (CallFunction|CheckReverseMovement)
    (else
      (Components|Movement|StopMovementImmediately _charactermovement))))

(event Custom|StartMovement
  (bind _returnvalue (Transformation|GetActorLocation))
  ;[1 0 0.006586] Animation by Timeline (DEPRECATED)
  (bind _alpha (Timeline|Timeline PlayFromStart)
    (:Update
      (Transformation|SetActorLocation (Math|Vector|MakeVector (- (.x _returnvalue) _alpha) (.y _returnvalue) (.z _returnvalue)) false false))))

(event Custom|CheckReverseMovement
  (if (>= (Math|Vector|Distance(Vector) (Transformation|GetActorLocation) (Variables|Default|GetInitialPosition)) 2e+02)
    (Components|Movement|StopMovementImmediately (Variables|Character|GetCharacterMovement))
    (Variables|Default|SetbCanMove false)
    (Utilities|FlowControl|FlipFlop
      (:A
        (Variables|Default|SetbIsReversed false))
      (:B
        (Variables|Default|SetbIsReversed true)))
    (Utilities|FlowControl|Delay 0.2)
    (Variables|Default|SetbCanMove true)))

(event EventAttack
  ;[0.7109 0 1] Attack Action
  (Variables|Default|SetbCanMove false)
  (|TriggerAnimationandsetloopfalse)
  (Default|Shoot (.AsBP%20Bullet%20Spawner (Utilities|Casting|CastToBP_BulletSpawner (Variables|/Script/Engine.ChildActorComponent|GetChildActor (Variables|Default|GetSpawner)))))
  (Utilities|FlowControl|Delay 0.5)
  (Variables|Default|SetbCanMove true))

(event EventTick
  (params (DeltaSeconds :type Float%20%28single-precision%29))
  (Utilities|FlowControl|Sequence
    (:then_0
      (CallFunction|Movement))))

(event EventBeginPlay
  ;[1 0 0.7266] Start
  (|CallParentFunction)
  (Components|Timeline|SetLooping (Variables|Default|GetSprite) true)
  (Variables|Default|SetInitialPosition (Transformation|GetActorLocation))
  (if (Variables|Default|GetbIsActive)
    (Utilities|Time|SetTimerbyEvent (delegate EventAttack) 3.0 true false 0.0 2.5)
    (CallFunction|Attack)))

(fn ConstructionScript
  (|CallParentFunction))

(fn IgnoreSight
  (Collision|SetCollisionEnabled (Variables|Default|GetSight) "NoCollision"))

(fn KillActor
  (|CallParentFunction))