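; Frag enemy child Blueprint that acts as a one-shot exploding hazard triggered when the player enters its Sight component.
; The first player overlap plays a Timeline that offsets the actor's Z from its current height on every update.
; When the Timeline finishes, the sprite switches to a non-looping explosion flipbook and the BP_BulletSpawner child actor shoots.
; The actor destroys itself once the flipbook finishes playing.
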(event OnFinishedPlaying(Sprite)
  ;[1 1 1] At Animation stop Destroy actor
  (Actor|DestroyActor))

(event OnComponentBeginOverlap(Sight)
  (params (OverlappedComponent :type Primitive%20Component%20Object%20Reference) (OtherActor :type Actor%20Object%20Reference) (OtherComp :type Primitive%20Component%20Object%20Reference) (OtherBodyIndex :type Integer) (bFromSweep :type Boolean) (SweepResult :type Hit%20Result%20Structure%20%28by%20ref%29))
  (bind _returnvalue (Transformation|GetActorLocation))
  (if (.bSuccess (Utilities|Casting|CastToBP_Core_Player OtherActor))
    (Utilities|FlowControl|DoOnce false
      (:Completed
        ;[1 1 1] Animation by Timeline
        (bind _alpha (Timeline|Timeline PlayFromStart)
          (:Update
            (Transformation|SetActorLocation (Math|Vector|MakeVector (.x _returnvalue) (.y _returnvalue) (+ _alpha (.z _returnvalue))) false false))
          (:Finished
            ;[1 1 1] Set not loop
            (Sprite|SetFlipbook (Variables|Default|GetSprite) "/Game/Enemies/Animations/Frag/FP_Enemy_Frag_Explode.FP_Enemy_Frag_Explode")
            (Components|Timeline|SetLooping (Variables|Default|GetSprite) false)
            (Default|Shoot (.AsBP%20Bullet%20Spawner (Utilities|Casting|CastToBP_BulletSpawner (Variables|/Script/Engine.ChildActorComponent|GetChildActor (Variables|Default|GetSpawner)))))))))))

(event EventBeginPlay)

(fn ConstructionScript
  (|CallParentFunction))