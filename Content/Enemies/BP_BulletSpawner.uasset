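; Enemy bullet spawner that fires BP_Bullet actors in a preset pattern on the X-Z plane when Shoot is called.
; Shoot switches on Pattern to four straight diagonals, two arcing upward diagonals, or an eight-way burst of diagonals and cardinals.
; Each pattern loops up to BulletCount, mapping the index to a fixed direction.
; Each bullet spawns at the spawner's location and receives its direction and movement type through BulletMovimentAction.
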(event Custom|Shoot
  (switch Utilities|FlowControl|Switch|SwitchonE_ShootPattern (Variables|Default|GetPattern)
    (:NewEnumerator2
      (|4DiagonalsStraight))
    (:NewEnumerator6
      (|2DiagonalsUpwithArc))
    (:NewEnumerator1
      (|360Straight))))

(event EventBeginPlay)

(event Collision|EventActorBeginOverlap
  (params (OtherActor :type Actor%20Object%20Reference)))

(event EventTick
  (params (DeltaSeconds :type Float%20%28single-precision%29)))

(fn ConstructionScript
  (Variables|Default|SetPattern (Variables|Default|GetPattern))
  (Variables|Default|SetBulletCount (Variables|Default|GetBulletCount)))

(fn ShootBullet)