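; Flipbook-animated enemy that periodically fires through a BP_BulletSpawner child actor while active.
; If active at BeginPlay, a looping timer triggers Attack, which switches to the attack flipbook, shoots, then sets CanMove after a delay.
; Finishing the attack animation restores the looping flipbook; Tick stops InterpToMovement simulation whenever the enemy is inactive.
; Timeline movement is deprecated, and the CanMove-driven movement logic is disconnected.
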(event OnFinishedPlaying(Sprite)
  (bind _sprite (Variables|Default|GetSprite))
  (Sprite|SetFlipbook _sprite "/Game/Enemies/Animations/FB_Enemy_360Frag.FB_Enemy_360Frag")
  (Components|Timeline|PlayfromStart _sprite)
  (Components|Timeline|SetLooping _sprite true))

(event Custom|Movement)

(event Custom|StartMovement
  (bind _returnvalue (Transformation|GetActorLocation))
  ;[1 0 0.006586] Animation by Timeline (DEPRECATED)
  (bind _alpha (Timeline|Timeline PlayFromStart)
    (:Update
      (Transformation|SetActorLocation (Math|Vector|MakeVector (- (.x _returnvalue) _alpha) (.y _returnvalue) (.z _returnvalue)) false false))))

(event EventBeginPlay
  ;[1 0 0.7266] Start
  (|CallParentFunction)
  (Components|Timeline|SetLooping (Variables|Default|GetSprite) true)
  (Variables|Default|SetInitialPosition (Transformation|GetActorLocation))
  (if (Variables|Default|GetbIsActive)
    (Utilities|Time|SetTimerbyEvent (delegate EventAttack) 3.0 true true)))

(event EventAttack
  ;[0.7109 0 1] Attack Action
  (bind _isactive (CallFunction|GetIsActive))
  (if _isactive
    (|TriggerAnimationandsetloopfalse_2)
    (Default|Shoot (.AsBP%20Bullet%20Spawner (Utilities|Casting|CastToBP_BulletSpawner (Variables|/Script/Engine.ChildActorComponent|GetChildActor (Variables|Default|GetSpawner)))))
    (Utilities|FlowControl|Delay 0.5)
    (Variables|Default|SetbCanMove true)))

(event EventTick
  (params (DeltaSeconds :type Float%20%28single-precision%29))
  (Utilities|FlowControl|Sequence
    (:then_0
      (bind _isactive (CallFunction|GetIsActive))
      (if (not _isactive)
        (Game|Components|ProjectileMovement|StopSimulating (Variables|Default|GetInterpToMovement) (Collision|MakeHitResult true false 0.0 0.0 "0, 0, 0" "0, 0, 0" "0,0,1" "0,0,1" 0 0))))))

(fn ConstructionScript
  (|CallParentFunction))