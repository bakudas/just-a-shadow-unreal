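; BP_SlashAttack_Base is a short-lived slash attack hitbox that destroys itself shortly after spawning.
; Its Sphere overlap ignores BP_Core_Player and applies fixed damage to actors implementing BPI_IDamageable, credited to the first player controller.
; A visibility sphere trace toward the victim, with debug drawing left on, supplies the impact point where it spawns BP_FX_Hit.
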(event OnComponentBeginOverlap(Sphere)
  (params (OverlappedComponent :type Primitive%20Component%20Object%20Reference) (OtherActor :type Actor%20Object%20Reference) (OtherComp :type Primitive%20Component%20Object%20Reference) (OtherBodyIndex :type Integer) (bFromSweep :type Boolean) (SweepResult :type Hit%20Result%20Structure%20%28by%20ref%29))
  (Utilities|Casting|CastToBP_Core_Player OtherActor
    (:CastFailed
      (if (Utilities|DoesObjectImplementInterface OtherActor "/Game/Game/Interfaces/BPI_IDamageable.BPI_IDamageable_C")
        (Game|Damage|ApplyDamage OtherActor 1e+01 (Game|GetPlayerController 0) 0 "/Script/Engine.DamageType")
        (bind _outhit (Collision|SphereTraceByChannel (Transformation|GetActorLocation) (Transformation|GetActorLocation OtherActor) 0.0 "TraceTypeQuery1" false 0 "ForDuration"))
        (Game|SpawnActorfromClass "/Game/Effects/BP_FX_Hit.BP_FX_Hit_C" (Math|Conversions|ToTransform(Vector) (.impactpoint _outhit)) "AlwaysSpawn" "MultiplyWithRoot" 0 0)))))

(event EventBeginPlay
  (Actor|SetLifeSpan 0.15))

(event Collision|EventActorBeginOverlap
  (params (OtherActor :type Actor%20Object%20Reference)))

(event EventTick
  (params (DeltaSeconds :type Float%20%28single-precision%29)))

(fn ConstructionScript)