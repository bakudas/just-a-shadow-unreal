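; Paper2D player character handling run, jump, slide, attack and dash input.
; Inputs and Tick set state flags, and UpdateAnimation selects a flipbook through AnimStateMachine, a priority branch function led by Dead, Attack and Slide.
; Tick also scales the sprite by X velocity for flipping and counts down cooldowns, while sliding resizes and offsets the capsule and sprite.
; Dash only sets a flag; slide impulse and paper-flip timelines are disconnected.
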(event Custom|UpdateAnimation
  ;[1 1 1] Update Animation
  (Variables|Character|SetIsMoving (!= (.x (Transformation|GetVelocity)) 0.0))
  (bind _outputflipbook (Character|AnimStateMachine))
  (Variables|Character|SetOutput%20Flipbook _outputflipbook)
  (Sprite|SetFlipbook (Variables|Character|GetSprite) _outputflipbook))

(event Input|EnhancedActionEvents|EnhancedInputActionIA_Attack_01
  (params (ActionValue :type Boolean) (ElapsedSeconds :type Float%20%28double-precision%29) (TriggeredSeconds :type Float%20%28double-precision%29) (InputAction :type Input%20Action%20Object%20Reference :default "/Game/Game/Inputs/IA_Attack_01.IA_Attack_01"))
  (bind _attackfx (Variables|Character|GetattackFX))
  (:Triggered
    ;[1 1 1] Check Attack
    (if (Math|Boolean|ANDBoolean (not (Variables|Character|GetIsJumping)) (not (Variables|Character|GetIsSliding)) (not (Variables|Character|GetIsFalling)))
      (Variables|Character|SetIsAttacking true)
      (Rendering|SetVisibility _attackfx true false)
      (CallFunction|UpdateAnimation :!label _label)))
  (:Canceled
    (Utilities|FlowControl|Delay 0.35 :!label _label_2)
    (Variables|Character|SetIsAttacking false)
    (Rendering|SetVisibility _attackfx false false)
    (goto _label))
  (:Completed
    (goto _label_2)))

(event Input|EnhancedActionEvents|EnhancedInputActionIA_Dash
  (params (ActionValue :type Boolean) (ElapsedSeconds :type Float%20%28double-precision%29) (TriggeredSeconds :type Float%20%28double-precision%29) (InputAction :type Input%20Action%20Object%20Reference :default "/Game/Game/Inputs/IA_Dash.IA_Dash"))
  ;[1 1 1] Dash
  (:Triggered
    (Variables|Character|SetIsDashing true)
    (CallFunction|UpdateAnimation :!label _label))
  (:Canceled
    (Variables|Character|SetIsDashing false :!label _label_2)
    (goto _label))
  (:Completed
    (goto _label_2)))

(event Input|EnhancedActionEvents|EnhancedInputActionIA_Slide
  (params (ActionValue :type Boolean) (ElapsedSeconds :type Float%20%28double-precision%29) (TriggeredSeconds :type Float%20%28double-precision%29) (InputAction :type Input%20Action%20Object%20Reference :default "/Game/Game/Inputs/IA_Slide.IA_Slide"))
  ;[1 1 1] Slide
  (:Triggered
    (Utilities|FlowControl|DoOnce false :!label _label
      (:Completed
        (if (Math|Boolean|ANDBoolean (<= (Variables|Character|GetSlideCooldown) 0.0) (Variables|Character|GetIsMoving) (Variables|Character|GetIsGrounded) (not (Variables|Character|GetIsFalling)))
          (Variables|Character|SetSlideCooldown 1.2)
          (Character|Slide true)))))
  (:Canceled
    (Character|GetUpfromSlide false :!label _label_2)
    (goto _label Reset))
  (:Completed
    (goto _label_2)))

(event Input|EnhancedActionEvents|EnhancedInputActionIA_Jump
  (params (ActionValue :type Boolean) (ElapsedSeconds :type Float%20%28double-precision%29) (TriggeredSeconds :type Float%20%28double-precision%29) (InputAction :type Input%20Action%20Object%20Reference :default "/Game/Game/Inputs/IA_Jump.IA_Jump"))
  ;[1 1 1] Jump and Falling
  (:Triggered
    (if (not (Variables|Character|GetIsSliding))
      (Character|Jump)
      (Variables|Character|SetIsGrounded false)
      (Sprite|SetFlipbook (Variables|Character|GetSprite) "/Game/Personagem/Animations/FB_Player_Jump.FB_Player_Jump")
      (Variables|Character|SetIsJumping true)
      (CallFunction|UpdateAnimation :!label _label)))
  (:Canceled
    (Character|StopJumping :!label _label_2)
    (if true
      (Variables|Character|SetIsJumping false)
      (goto _label)))
  (:Completed
    (goto _label_2)))

(event Input|EnhancedActionEvents|EnhancedInputActionIA_Run
  (params (ActionValue :type Float%20%28double-precision%29) (ElapsedSeconds :type Float%20%28double-precision%29) (TriggeredSeconds :type Float%20%28double-precision%29) (InputAction :type Input%20Action%20Object%20Reference :default "/Game/Game/Inputs/IA_Run.IA_Run"))
  ;[1 1 1] Basic Movement
  (if (not (Variables|Character|GetIsAttacking))
    (Variables|Character|SetDirection ActionValue)
    (Class|PawnMovementComponent|AddInputVector (Variables|Character|GetCharacterMovement) (Math|Vector|MakeVector ActionValue 0.0 0.0) false)
    (CallFunction|UpdateAnimation)))

(event EventTick
  (params (DeltaSeconds :type Float%20%28single-precision%29))
  (bind _returnvalue (Transformation|GetVelocity))
  (Utilities|FlowControl|Sequence
    (:then_0
      ;[1 1 1] Is Falling
      (bind _output_get (Variables|Character|SetIsFalling (< (.z (Transformation|GetVelocity)) 0.0)))
      (if _output_get
        (Variables|Character|SetIsGrounded false)
        (CallFunction|UpdateAnimation)))
    (:then_1
      ;[1 1 1] Horizontal Flip Sprite
      (if (!= (.x _returnvalue) 0.0)
        (Class|SceneComponent|AddLocalTransform (Variables|Character|GetSprite) (Math|Transform|MakeTransform "0, 0, 0" "0, 0, 0" (Math|Vector|MakeVector (* (.x _returnvalue) (Variables|Character|GetScaleX)) 1.0 1.0)) false false)))
    (:then_2
      ;[1 1 1] Slide Cooldown
      (if (> (Variables|Character|GetSlideCooldown) 0.0)
        (Variables|Character|SetSlideCooldown (- (Variables|Character|GetSlideCooldown) DeltaSeconds))))
    (:then_3
      ;[1 1 1] Attack Cooldown
      (if (> (Variables|Character|GetAttackCooldown) DeltaSeconds)
        (Variables|Character|SetAttackCooldown (- (Variables|Character|GetAttackCooldown) 1.0))))))

(event EventOnLanded
  (params (Hit :type Hit%20Result%20Structure%20%28by%20ref%29))
  ;[1 1 1] Set Grounded
  (Variables|Character|SetIsGrounded true)
  (CallFunction|UpdateAnimation))

(fn ConstructionScript)

(fn AnimStateMachine
  (if (Variables|Character|GetIsDead)
    (Variables|Character|SetAnimationState "NewEnumerator6")
    (switch Utilities|FlowControl|Switch|SwitchonAnimationState (Variables|Character|GetAnimationState) :!label _label
      (:NewEnumerator0
        _)
      (:NewEnumerator1
        _)
      (:NewEnumerator2
        _)
      (:NewEnumerator4
        _)
      (:NewEnumerator3
        _)
      (:NewEnumerator5
        _)
      (:NewEnumerator6
        _))
    (return (Utilities|Select :Index (Variables|Character|GetAnimationState) :NewEnumerator0 (Variables|Character|GetIdleFlipbook) :NewEnumerator1 (Variables|Character|GetRunFlipbook) :NewEnumerator2 (Variables|Character|GetJumpFlipbook) :NewEnumerator4 (Variables|Character|GetFallingFlipbook) :NewEnumerator3 (Variables|Character|GetSlideFlipbook) :NewEnumerator5 (Variables|Character|GetAttackFlipbook) :NewEnumerator6 (Variables|Character|GetDeadFlipbook)))
    (elif (Variables|Character|GetIsAttacking)
      (Variables|Character|SetAnimationState "NewEnumerator5")
      (goto _label)
      (elif (and (Variables|Character|GetIsSliding) (not (Variables|Character|GetIsJumping)))
        (Variables|Character|SetAnimationState "NewEnumerator3")
        (goto _label)
        (elif (Variables|Character|GetIsGrounded)
          (if (Variables|Character|GetIsMoving)
            (Variables|Character|SetAnimationState "NewEnumerator1")
            (goto _label)
            (else
              (Variables|Character|SetAnimationState "NewEnumerator0")
              (goto _label)))
          (elif (Variables|Character|GetIsFalling)
            (Variables|Character|SetAnimationState "NewEnumerator4")
            (goto _label)
            (elif (Variables|Character|GetIsJumping)
              (Variables|Character|SetAnimationState "NewEnumerator2")
              (goto _label))))))))

(fn Slide
  (params (Slide :type Boolean))
  (bind _capsulecomponent (Variables|Collision|GetCapsuleComponent))
  (bind _relativelocation (Variables|/Script/Engine.SceneComponent|GetRelativeLocation _capsulecomponent))
  (Utilities|FlowControl|Sequence
    (:then_0
      (Variables|Character|SetIsSliding true)
      ;[1 1 1] Set Capsule Collider Height
      (Components|Capsule|SetCapsuleHalfHeight (Variables|Collision|GetCapsuleComponent) (Variables|Character|GetSlideCapsuleHeight) true)
      ;[1 1 1] Set Sprite Relative Location
      (Transformation|SetRelativeLocation (Variables|Character|GetSprite) (Math|Vector|MakeVector 0.0 0.0 (Variables|Character|GetSlideSpriteLocation)) false false)
      ;[1 1 1] Set Capsule Offset Location
      (Transformation|SetRelativeLocation _capsulecomponent (Math|Vector|MakeVector (.x _relativelocation) (.y _relativelocation) (+ (* (Variables|Character|GetOffsetRelativeLocation) -1.0) (.z _relativelocation))) false false))))

(fn GetUpfromSlide
  (params (Slide :type Boolean))
  (bind _capsulecomponent (Variables|Collision|GetCapsuleComponent))
  (bind _relativelocation (Variables|/Script/Engine.SceneComponent|GetRelativeLocation _capsulecomponent))
  (Variables|Character|SetIsSliding false)
  (Components|Capsule|SetCapsuleHalfHeight (Variables|Collision|GetCapsuleComponent) (Variables|Character|GetStandUpCapsuleHeight) true)
  (Transformation|SetRelativeLocation (Variables|Character|GetSprite) (Math|Vector|MakeVector 0.0 0.0 (Variables|Character|GetStandUpSpriteLocation)) false false)
  (Transformation|SetRelativeLocation _capsulecomponent (Math|Vector|MakeVector (.x _relativelocation) (.y _relativelocation) (+ (* (Variables|Character|GetOffsetRelativeLocation) 1.0) (.z _relativelocation))) false false))